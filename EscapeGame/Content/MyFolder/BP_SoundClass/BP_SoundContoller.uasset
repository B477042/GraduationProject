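; BP_SoundContoller is a Blueprint that applies the player's saved options when play begins.
; It loads the options through EGGameInstance, then overrides BGM, SFX, UI and Voice sound class volumes in a sound mix, each slider scaled by the master value.
; It also sets fullscreen mode and resolution on GameUserSettings, with no visible ApplySettings call or sound mix push.
; Invalid options data only prints an error message.
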(event `self.ReceiveBeginPlay`
  (bind _aseggame_instance (cast `EGGameInstance` (`GameplayStatics.GetGameInstance`)))
  (bind _returnvalue (`EGGameInstance.LoadOptions` _aseggame_instance))
  (`self.Load Options` _returnvalue))

(fn `Load Options`
  (params (LoadInstance :type "OptionSaveGame Object Reference"))
  (bind _sld_mastervalue (`OptionSaveGame.sld_MasterValue` LoadInstance))
  (`/Engine/EditorBlueprintResources/StandardMacros.IsValid` LoadInstance
    (:`Is Valid`
      ;[1 1 1] Sound Settings
      (`GameplayStatics.SetSoundMixClassOverride` "/Game/MyFolder/BP_SoundClass/BP_SM_EGSoundMix.BP_SM_EGSoundMix" "/Game/MyFolder/BP_SoundClass/BP_SC_BGM.BP_SC_BGM" (* _sld_mastervalue (`OptionSaveGame.sld_BGMValue` LoadInstance)))
      (`GameplayStatics.SetSoundMixClassOverride` "/Game/MyFolder/BP_SoundClass/BP_SM_EGSoundMix.BP_SM_EGSoundMix" "/Game/MyFolder/BP_SoundClass/BP_SC_SFX.BP_SC_SFX" (* (`OptionSaveGame.sld_SEValue` LoadInstance) _sld_mastervalue))
      (`GameplayStatics.SetSoundMixClassOverride` "/Game/MyFolder/BP_SoundClass/BP_SM_EGSoundMix.BP_SM_EGSoundMix" "/Game/MyFolder/BP_SoundClass/BP_SC_UISound.BP_SC_UISound" (* (`OptionSaveGame.sld_UIValue` LoadInstance) _sld_mastervalue))
      (`GameplayStatics.SetSoundMixClassOverride` "/Game/MyFolder/BP_SoundClass/BP_SM_EGSoundMix.BP_SM_EGSoundMix" "/Game/MyFolder/BP_SoundClass/BP_SC_Voice.BP_SC_Voice" (* (`OptionSaveGame.sld_VoiceValue` LoadInstance) _sld_mastervalue))
      ;[1 1 1] Screen Settings
      (bind _returnvalue (`GameUserSettings.GetGameUserSettings`))
      (`GameUserSettings.SetFullscreenMode` _returnvalue (`OptionSaveGame.WindowMode` LoadInstance))
      (`GameUserSettings.SetScreenResolution` _returnvalue (`OptionSaveGame.ScreenResoultion` LoadInstance)))
    (:`Is Not Valid`
      (`KismetSystemLibrary.PrintString` "Fail to load options data" true true (struct :`R` 1.0 :`B` 0.086574 :`A` 1.0)))))

(fn `UserConstructionScript`)