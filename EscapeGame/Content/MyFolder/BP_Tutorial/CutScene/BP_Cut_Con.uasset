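; Player controller for tutorial cutscenes that shows a dialogue widget with UI-only input and a visible cursor.
; On BeginPlay it copies the next stage and act from the level's Promptor actor into the widget, then loads up to six numbered data table rows.
; The widget's Next and Prev delegates step through lines, updating talker and text.
; Next opens the next level once the count passes MaxCount.
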(event `self.ReceiveBeginPlay`
  (bind _returnvalue (`|CreateWidget` (`self.DialogueClass`)))
  (bind _output_get (set `self.UI_Dialogue` _returnvalue))
  (`UserWidget.AddToViewport` _output_get 0)
  (`WidgetBlueprintLibrary.SetInputMode_UIOnlyEx` self _output_get)
  (set `self.bShowMouseCursor` true)
  (bind _returnvalue_2 (`GameplayStatics.GetActorOfClass` "/Script/EscapeGame.Promptor"))
  (bind _asdialogue_widget (cast `DialogueWidget` (`self.UI_Dialogue`)))
  (set `DialogueWidget.NextStage` (`Promptor.NextStage` _returnvalue_2) _asdialogue_widget)
  (set `DialogueWidget.n_Act` (`Promptor.n_Act` _returnvalue_2) _asdialogue_widget)
  (`self.Load Dialogue`)
  (`self.PrintDialogue`)
  (add `DialogueWidget.OnClickNextDelegate` _asdialogue_widget (delegate `OnClickNextDelegate_Event_0`))
  (add `DialogueWidget.OnClickPrevDelegate` _asdialogue_widget (delegate `OnClickPrevDelegate_Event_0`)))

(event `OnClickPrevDelegate_Event_0`
  (bind _logcount (`self.LogCount`))
  (if (not (>= 0 _logcount))
    (set `self.LogCount` (- _logcount 1))
    (`self.PrintDialogue`)))

(event `OnClickNextDelegate_Event_0`
  (bind _logcount (`self.LogCount`))
  (if (>= (`self.MaxCount`) _logcount)
    (set `self.LogCount` (+ _logcount 1))
    (`self.PrintDialogue`)
    (else
      (`GameplayStatics.OpenLevel` (`DialogueWidget.NextStage` (stale `self.ReceiveBeginPlay` _asdialogue_widget))))))

(fn `Load Dialogue`
  (locals (Index :type Integer))
  (bind _dialogue_data_table (`self.Dialogue Data Table`))
  (`/Engine/EditorBlueprintResources/StandardMacros.IsValid` _dialogue_data_table
    (:`Is Valid`
      (set `local.Index` 0)
      (for _ (range 6)
        (bind _returnvalue (`|GetDataTableRow` _dialogue_data_table (`KismetStringLibrary.Conv_StringToName` (`KismetStringLibrary.Conv_IntToString` (`local.Index`))))
          (:`then`
            (`KismetArrayLibrary.Array_Add` (`self.Dialouges`) _returnvalue)
            (set `local.Index` (+ (`local.Index`) 1))))))))

(fn `PrintDialogue`
  (locals (NewLocalVar_0 :type "EditableTextStyle Structure" :default (struct :`Font` (struct :`OutlineSettings` (struct :`OutlineColor` (struct :`A` 1.0)) :`TypefaceFontName` "Regular" :`Size` 9) :`ColorAndOpacity` (struct :`SpecifiedColor` (struct :`R` 1.0 :`G` 0.378145 :`B` 0.248122 :`A` 1.0) :`ColorUseRule` "UseColor_Specified") :`BackgroundImageSelected` (struct :`ImageSize` (32.0 32.0) :`Margin` (struct) :`TintColor` (struct :`SpecifiedColor` (struct :`R` 1.0 :`G` 1.0 :`B` 1.0 :`A` 1.0) :`ColorUseRule` "UseColor_Specified") :`UVRegion` (struct :`Min` (0.0 0.0) :`Max` (0.0 0.0)) :`DrawAs` "Image" :`Tiling` "NoTile" :`Mirroring` "NoMirror" :`ImageType` "NoImage") :`BackgroundImageComposing` (struct :`ImageSize` (32.0 32.0) :`Margin` (struct) :`TintColor` (struct :`SpecifiedColor` (struct :`R` 1.0 :`G` 1.0 :`B` 1.0 :`A` 1.0) :`ColorUseRule` "UseColor_Specified") :`UVRegion` (struct :`Min` (0.0 0.0) :`Max` (0.0 0.0)) :`DrawAs` "Image" :`Tiling` "NoTile" :`Mirroring` "NoMirror" :`ImageType` "NoImage") :`CaretImage` (struct :`ImageSize` (32.0 32.0) :`Margin` (struct) :`TintColor` (struct :`SpecifiedColor` (struct :`R` 1.0 :`G` 1.0 :`B` 1.0 :`A` 1.0) :`ColorUseRule` "UseColor_Specified") :`UVRegion` (struct :`Min` (0.0 0.0) :`Max` (0.0 0.0)) :`DrawAs` "Image" :`Tiling` "NoTile" :`Mirroring` "NoMirror" :`ImageType` "NoImage"))))
  (bind _ui_dialogue (`self.UI_Dialogue`))
  (bind (_dialogue _talker) (break `DialogueTableRow` (`|GetArrayItem` (`self.Dialouges`) (`self.LogCount`))))
  (`/Engine/EditorBlueprintResources/StandardMacros.IsValid` _ui_dialogue
    (:`Is Valid`
      (bind _asdialogue_widget (cast `DialogueWidget` _ui_dialogue))
      (`DialogueWidget.SetTalkerName` _asdialogue_widget _talker)
      (`EditableText.SetText` (`DialogueWidget.TextDiagram` _asdialogue_widget) (`KismetTextLibrary.Conv_StringToText` _dialogue)))))

(fn `UserConstructionScript`)