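; Tutorial notification actor that, on BeginPlay, creates a tutorial widget to show a title, description and image.
; The NotifyType map lookup picks a DTTutorial row, whose text and image path fill the widget.
; Filling depends on IsVisible, though this graph never adds the widget to the viewport.
; The image cast runs on the async load's immediate exec pin; Completed only prints a failure message.
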(event `self.ReceiveBeginPlay`
  (bind _tutowidget (`self.TutoWidget`))
  (bind _returnvalue (`|CreateWidget` (`self.Tuto Widget Class`) (`GameplayStatics.GetPlayerController` 0)))
  (bind _output_get (set `self.TutoWidget` _returnvalue))
  (if (`Widget.IsVisible` _output_get)
    (bind _returnvalue_2 (`|GetDataTableRow` (`self.DT_Tutorial`) (`BlueprintMapLibrary.Map_Find` (`self.SetOfTypesOfNotifications`) (`self.NotifyType`)))
      (:`then`
        (bind (_notifyname _notifytittle _describe _gifpath) (break `TutorialDataTable` _returnvalue_2))
        (`TextBlock.SetText` (`TutorialWidget.Txt_NotifyTittle` _tutowidget) _notifytittle)
        (`MultiLineEditableTextBox.SetText` (`TutorialWidget.Txt_Describe` _tutowidget) _describe)
        (bind _object (`|LoadAsset` (`KismetSystemLibrary.Conv_SoftObjPathToSoftObjRef` _gifpath))
          (:`then`
            (bind _astexture_2d (cast `Texture2D` _object)
              (:`then`
                (`Image.SetBrushFromTexture` (`TutorialWidget.GIF` _tutowidget) _astexture_2d false)
                (`KismetSystemLibrary.PrintString` "widget done"))
              (:`CastFailed`
                (`KismetSystemLibrary.PrintString` "fail to find widget 2d"))))
          (:`Completed`
            (`KismetSystemLibrary.PrintString` "fail to find widget async"))))
      (:`RowNotFound`
        (`KismetSystemLibrary.PrintString` "Fail to find widget row")))
    (else
      (`KismetSystemLibrary.PrintString` "Fail to create widget"))))

(event `self.ReceiveActorBeginOverlap`
  (params (OtherActor :type "Actor Object Reference")))

(fn `UserConstructionScript`)