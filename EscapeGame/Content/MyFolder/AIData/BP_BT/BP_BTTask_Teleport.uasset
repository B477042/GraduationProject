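; Behavior tree task meant to teleport an EnemyBossCharacter to a random spot around the blackboard TargetPos.
; CalcNewPos adds a random horizontal offset scaled by TeleportDistance, then CheckNewPos line-traces upward from that point.
; A passing check triggers TeleportTo with the current rotation and finishes with its result.
; As written, both CheckNewPos branches return false, so the task fails without teleporting.
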(event `self.ReceiveExecuteAI`
  (params (OwnerController :type "AIController Object Reference") (ControlledPawn :type "Pawn Object Reference"))
  (bind _asenemy_boss_character (cast `EnemyBossCharacter` ControlledPawn))
  (bind _returnvalue (`self.Calc New pos` OwnerController)) ; 플레이어 주변 Teleport Distance 이내의 위치를 임의로 출력해낸다.
  (bind _output_get (set `self.tempTelePos` _returnvalue))
  (bind _result (`self.Check new pos` _output_get))
  (if _result
    (bind _returnvalue_2 (`EnemyBossCharacter.TeleportTo` _asenemy_boss_character _output_get (`Actor.K2_GetActorRotation` _asenemy_boss_character) false false))
    (`self.FinishExecute` _returnvalue_2)
    (else
      (`self.FinishExecute` false))))

(fn `Calc New pos`
  (params (Target :type "Actor Object Reference"))
  (returns (ReturnValue :type "Vector Structure"))
  (return (+ (`BlackboardComponent.GetValueAsVector` (`AIBlueprintHelperLibrary.GetBlackboard` Target) (`self.TargetPos`)) (`KismetMathLibrary.MakeVector` (.x (* (`KismetMathLibrary.RandomUnitVector`) (`self.Teleport Distance`))) (.y (* (`KismetMathLibrary.RandomUnitVector`) (`self.Teleport Distance`)))))))

(fn `Check new pos`
  (params (Start :type "Vector Structure"))
  (returns (result :type Boolean))
  (locals (NewLocalVar_0 :type "Array of Actor Object Reference") (NewLocalVar_1 :type "Array of Actor Object Reference") (NewLocalVar_2 :type "Array of EObjectTypeQuery Enum"))
  (bind (_outhit _returnvalue) (`KismetSystemLibrary.LineTraceSingleForObjects` Start (+ Start (0.0 0.0 100.0)) (`local.NewLocalVar_2`)))
  (if _returnvalue
    (return false)
    (else
      (`KismetSystemLibrary.PrintString` "false")
      (return false))))