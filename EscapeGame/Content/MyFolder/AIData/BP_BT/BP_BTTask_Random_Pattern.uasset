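; Behavior tree task that randomly picks a boss's next BehaviorPattern from its Blackboard.
; When MP is zero or below, it sets one fixed pattern and finishes as failed.
; Otherwise it rolls an integer, writes one of four patterns and succeeds, looping back to reroll on the unmapped value.
; A time-seeded random stream is set before each roll, but the roll itself does not use that stream.
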(event `self.ReceiveExecuteAI`
  (params (OwnerController :type "AIController Object Reference") (ControlledPawn :type "Pawn Object Reference"))
  (bind _returnvalue (`AIBlueprintHelperLibrary.GetBlackboard` OwnerController))
  (bind _seconds (`GameplayStatics.GetAccurateRealTime`))
  (if (<= (`BlackboardComponent.GetValueAsFloat` _returnvalue (`self.MP`)) 0.0)
    (`BlackboardComponent.SetValueAsEnum` _returnvalue (`self.BehaviorPattern`) (enumliteral `/Game/MyFolder/AIData/BB_Enum/StateNameForBoss` "NewEnumerator2"))
    (`self.FinishExecute` false)
    (else
      (`KismetMathLibrary.SetRandomStreamSeed` (`KismetMathLibrary.MakeRandomStream` _seconds) _seconds :!label _label)
      (switch `int` (`KismetMathLibrary.RandomIntegerInRange` 0 4)
        (:`Default`
          (goto _label))
        (:`0`
          (`BlackboardComponent.SetValueAsEnum` _returnvalue (`self.BehaviorPattern`) (enumliteral `/Game/MyFolder/AIData/BB_Enum/StateNameForBoss` "NewEnumerator1")))
        (:`1`
          (`BlackboardComponent.SetValueAsEnum` _returnvalue (`self.BehaviorPattern`) (enumliteral `/Game/MyFolder/AIData/BB_Enum/StateNameForBoss` "NewEnumerator4")))
        (:`2`
          (`BlackboardComponent.SetValueAsEnum` _returnvalue (`self.BehaviorPattern`) (enumliteral `/Game/MyFolder/AIData/BB_Enum/StateNameForBoss` "NewEnumerator5")))
        (:`3`
          (`BlackboardComponent.SetValueAsEnum` _returnvalue (`self.BehaviorPattern`) (enumliteral `/Game/MyFolder/AIData/BB_Enum/StateNameForBoss` "NewEnumerator6"))))
      (`self.FinishExecute` true))))