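; Behavior Tree task that computes a back-step point for the AI-controlled character and writes it to the Blackboard.
; The point is the sum of the Blackboard target position, the pawn's forward vector scaled by BackStepValue, and the character's own location.
; It prints the character location and result for debugging, then finishes with success; a failed Character cast stops it before finishing.
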(event `self.ReceiveExecuteAI`
  (params (OwnerController :type "AIController Object Reference") (ControlledPawn :type "Pawn Object Reference"))
  (bind _returnvalue (`AIBlueprintHelperLibrary.GetBlackboard` OwnerController))
  (bind _output_get (set `self.VTargetPos` (`BlackboardComponent.GetValueAsVector` _returnvalue (`self.NTargetPos`)))) ; TargetPos
  (bind _output_get_2 (set `self.FV` (`Actor.GetActorForwardVector` ControlledPawn))) ; Owner의 FV
  (bind _ascharacter (cast `Character` ControlledPawn))
  (bind _returnvalue_2 (`Actor.K2_GetActorLocation` _ascharacter))
  (bind _output_get_3 (set `self.BackStepPoint` (+ (+ _output_get (* _output_get_2 (`self.BackStepValue`))) _returnvalue_2)))
  (`KismetSystemLibrary.PrintString` "My Pos")
  (`KismetSystemLibrary.PrintString` (`KismetStringLibrary.Conv_VectorToString` _returnvalue_2))
  (`KismetSystemLibrary.PrintString` "BackStep Pos")
  (`KismetSystemLibrary.PrintString` (`KismetStringLibrary.Conv_VectorToString` _output_get_3))
  (`BlackboardComponent.SetValueAsVector` _returnvalue (`self.NBackStepPoint`) _output_get_3)
  (`self.FinishExecute` true))