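; Behavior tree service that, by its name, moves an AI character to a backstep point during a jump or dodge.
; Each AI tick it prints "Jumping" and measures the distance from the Character to the Backstep blackboard vector.
; It offsets the actor along its forward vector, scaled by that distance and delta time, without sweeping.
; The point sets only the step size, never the direction.
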(event `self.ReceiveTickAI`
  (params (OwnerController :type "AIController Object Reference") (ControlledPawn :type "Pawn Object Reference") (DeltaSeconds :type "Float (single-precision)"))
  (`KismetSystemLibrary.PrintString` "Jumping")
  (bind _ascharacter (cast `Character` ControlledPawn))
  (`Actor.K2_AddActorWorldTransform` _ascharacter (`KismetMathLibrary.Conv_VectorToTransform` (* (`Actor.GetActorForwardVector` _ascharacter) (* (`KismetMathLibrary.Vector_Distance` (`Actor.K2_GetActorLocation` _ascharacter) (`BlackboardComponent.GetValueAsVector` (`AIBlueprintHelperLibrary.GetBlackboard` OwnerController) (`self.backstep`))) (* DeltaSeconds 3.0)))) false false))