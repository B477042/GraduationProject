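; Tutorial player character that finds a nearby NPC to act as the dialogue talker.
; On BeginPlay it moves to a stored position and rotation, then runs a sphere overlap and stores the first NPCCharacter found as Talkers.
; SetTalkerToUi, not called in this Blueprint, passes that NPC and its name to the tutorial controller's dialogue UI.
; Its UI validity check runs only when the controller cast fails.
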(event `self.ReceiveBeginPlay`
  (`self.K2_SetActorLocationAndRotation` (`self.Pos`) (`self.Rot`))
  (`self.Scan  NPC`))

(fn `Scan  NPC`
  (returns (NewParam :type "NPCCharacter Object Reference"))
  (locals (NewLocalVar_0 :type "Array of EObjectTypeQuery Enum"))
  (bind _outactors (`KismetSystemLibrary.SphereOverlapActors` (`self.K2_GetActorLocation`) 2000.0 (`local.NewLocalVar_0`)))
  (for _array_element _outactors
    (bind _asnpccharacter (cast `NPCCharacter` _array_element))
    (bind _output_get (set `self.Talkers` _asnpccharacter))
    (`KismetSystemLibrary.PrintString` "Scan Success")
    (return _output_get)))

(fn `Set Talker To Ui`
  (bind _talkers (`self.Talkers`))
  (bind _asbp_tutorial_controller (cast `/Game/MyFolder/BP_Tutorial/BP_TutorialController` (`self.GetController`))
    (:`then`
      (bind _ui_dialogue (`/Game/MyFolder/BP_Tutorial/BP_TutorialController.UI_Dialogue` _asbp_tutorial_controller))
      (`DialogueWidget.SetTalker` _ui_dialogue _talkers (`KismetTextLibrary.Conv_StringToText` (`NPCCharacter.Name` _talkers)) :!label _label)
      (`KismetSystemLibrary.PrintText` "SUCCCCCCCCC"))
    (:`CastFailed`
      (`/Engine/EditorBlueprintResources/StandardMacros.IsValid` _ui_dialogue
        (:`Is Valid`
          (goto _label))
        (:`Is Not Valid`
          (`KismetSystemLibrary.PrintString` "NOT VAILED"))))))

(fn `UserConstructionScript`)