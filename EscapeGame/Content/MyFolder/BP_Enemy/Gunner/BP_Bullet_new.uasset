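; BP_Bullet_new is a Gunner enemy projectile that stays hidden until Fired gives it a direction, shows it and enables its trigger collision.
; Tick moves it without sweep by BulletSpeed plus DeltaSeconds times Accel, so speed is frame-rate dependent and never accumulates.
; Any overlap applies damage, stops and hides the bullet, disables collision and plays HitEffect until deactivation.
; It is never destroyed, so Fired can reuse it.
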(event `self.ReceiveTick`
  (params (DeltaSeconds :type "Float (single-precision)"))
  (if (`self.isfired`)
    (`self.K2_SetActorLocation` (+ (* (`self.Direction`) (+ (* DeltaSeconds (`self.Accel`)) (`self.BulletSpeed`))) (`self.K2_GetActorLocation`)))))

(event `self.HitCollision.OnComponentBeginOverlap`
  (params (OverlappedComponent :type "PrimitiveComponent Object Reference") (OtherActor :type "Actor Object Reference") (OtherComp :type "PrimitiveComponent Object Reference") (OtherBodyIndex :type Integer) (bFromSweep :type Boolean) (SweepResult :type "HitResult Structure (by ref)"))
  (bind _hiteffect (`self.HitEffect`))
  (if true
    (`GameplayStatics.ApplyDamage` OtherActor (`self.dmage`) null self)
    (`KismetSystemLibrary.PrintString` (`KismetSystemLibrary.GetObjectName` OtherActor))
    (set `self.isfired` false)
    (`SceneComponent.SetHiddenInGame` (`self.BulletBody`) true true)
    (`SceneComponent.SetHiddenInGame` _hiteffect false false)
    (`ActorComponent.Activate` _hiteffect false)
    (`PrimitiveComponent.SetCollisionProfileName` (`self.HitCollision`) "NoCollision")))

(event `self.HitEffect.OnComponentDeactivated`
  (params (Component :type "ActorComponent Object Reference"))
  (`SceneComponent.SetHiddenInGame` (`self.HitEffect`) true false))

(fn `Fired`
  (params (inputDirection :type "Vector Structure"))
  (set `self.Direction` inputDirection)
  (set `self.isfired` true)
  (`SceneComponent.SetHiddenInGame` (`self.BulletBody`) false true)
  (`PrimitiveComponent.SetCollisionProfileName` (`self.HitCollision`) "OnTrapTrigger"))

(fn `UserConstructionScript`
  (`SceneComponent.SetHiddenInGame` (`self.HitEffect`) true true)
  (`SceneComponent.SetHiddenInGame` (`self.BulletBody`) true true)
  (`SceneComponent.SetHiddenInGame` (`self.FlyEffect`) true true)
  (`self.K2_SetActorLocation` (0.0 0.0 0.0)))