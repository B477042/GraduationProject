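; Behavior tree service that keeps the AI's target position in the blackboard up to date.
; On each AI tick it reads the TargetPlayer object from the owner controller's blackboard and casts it to Character.
; It then writes that character's actor location to the TargetPos key, leaving the key unchanged when the controller or target is invalid or not a Character.
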(event `self.ReceiveTickAI`
  (params (OwnerController :type "AIController Object Reference") (ControlledPawn :type "Pawn Object Reference") (DeltaSeconds :type "Float (single-precision)"))
  (bind _returnvalue (`AIBlueprintHelperLibrary.GetBlackboard` OwnerController))
  (bind _returnvalue_2 (`BlackboardComponent.GetValueAsObject` _returnvalue (`self.TargetPlayer`)))
  (if (`KismetSystemLibrary.IsValid` OwnerController)
    (if (`KismetSystemLibrary.IsValid` _returnvalue_2)
      (bind _ascharacter (cast `Character` _returnvalue_2))
      (`BlackboardComponent.SetValueAsVector` _returnvalue (`self.TargetPos`) (`Actor.K2_GetActorLocation` _ascharacter)))))