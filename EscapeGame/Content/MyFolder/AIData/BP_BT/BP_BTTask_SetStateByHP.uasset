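; Behavior tree task that picks the enemy boss's behavior pattern from its current HP.
; It casts the controlled pawn to EnemyBossCharacter and reads HP from its Stat.
; Below a fixed threshold it sets the BehaviorPattern blackboard enum to a regroup state, otherwise to idle, then finishes successfully.
; A failed cast stops execution without calling FinishExecute.
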(event `self.ReceiveExecuteAI`
  (params (OwnerController :type "AIController Object Reference") (ControlledPawn :type "Pawn Object Reference"))
  (bind _returnvalue (`AIBlueprintHelperLibrary.GetBlackboard` OwnerController))
  (bind _behaviorpattern (`self.BehaviorPattern`))
  (bind _asenemy_boss_character (cast `EnemyBossCharacter` ControlledPawn))
  (if (> 40.0 (`StatComponent.GetHP` (`EnemyBossCharacter.Stat` _asenemy_boss_character)))
    (`BlackboardComponent.SetValueAsEnum` _returnvalue _behaviorpattern (enumliteral `/Game/MyFolder/AIData/BP_BT/StateNameForBoss` "NewEnumerator2")) ; 40보다 작다면 재정비를 해야된다
    (else
      (`BlackboardComponent.SetValueAsEnum` _returnvalue _behaviorpattern (enumliteral `/Game/MyFolder/AIData/BP_BT/StateNameForBoss` "NewEnumerator0")) ; 40보다 크다면 idle 상태로 해둡니다
    ))
  (`self.FinishExecute` true))